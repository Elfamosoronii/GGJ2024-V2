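; Boss Blueprint that shows its dialogue lines on screen through repeated Talk events.
; Each Talk increments TalkIndex and compares it against the length of the DIalogue array.
; While within range, it lazily creates and displays a Wid_Dialogue widget, then sets its text from the entry at TalkRef, a separate variable from the counter.
; Past the end, it removes the widget from its parent.
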(event EventTalk
  (bind _result (Math|Integer|IncrementInt (Variables|Default|GetTalkIndex))
    (:%20%20
      (if (<= _result (Utilities|Array|Length (Variables|Default|GetDIalogue)))
        (Variables|Default|GetUI
          (:then
            _)
          (:else
            (bind _returnvalue (UserInterface|CreateWidget "/Game/Prog/Dialogue/Wid_Dialogue.Wid_Dialogue_C" (Game|GetPlayerController 0)))
            (bind _output_get (Variables|Default|SetUI _returnvalue))
            (UserInterface|Viewport|AddtoViewport _output_get 0)))
        (Rendering|Components|TextRender|SetText (Variables|/Game/Prog/Dialogue/Wid_Dialogue.Wid_Dialogue_C|GetTalkText (Variables|Default|GetUI)) (Utilities|Text|ToText(String) (Utilities|Array|Get(acopy) (Variables|Default|GetDIalogue) (Variables|Default|GetTalkRef))))
        (else
          (Widget|RemovefromParent (Variables|Default|GetUI)))))))

(fn ConstructionScript)